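; Endless-runner track tile that populates three lanes with random obstacles, coins or magnet and boots pickups on BeginPlay.
; SpawnObstacle chains weighted checks per lane, each with a fresh random roll, so a lane where all checks fail also leaves later lanes empty.
; When the character overlaps Collision, it has the game mode spawn another tile, adds multiplied score, raises walk speed within a clamp, then destroys itself after a delay.
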(event `self.ReceiveBeginPlay`
  (`self.SpawnObstacle`))

(event `self.Collision.OnComponentBeginOverlap`
  (params (OverlappedComponent :type "PrimitiveComponent Object Reference") (OtherActor :type "Actor Object Reference") (OtherComp :type "PrimitiveComponent Object Reference") (OtherBodyIndex :type Integer) (bFromSweep :type Boolean) (SweepResult :type "HitResult Structure (by ref)"))
  (bind _asbp_character (cast `/Game/Blueprints/BP_Character` OtherActor))
  (bind _asbp_gameplay_gm (cast `/Game/Blueprints/BP_GameplayGM` (`GameplayStatics.GetGameMode`)))
  (`/Game/Blueprints/BP_GameplayGM.SpawnTile` _asbp_gameplay_gm)
  (set `/Game/Blueprints/BP_GameplayGM.Score` (+ (`/Game/Blueprints/BP_GameplayGM.Score` _asbp_gameplay_gm) (* 1 (`/Game/Blueprints/BP_GameplayGM.ScoreMultiplier` _asbp_gameplay_gm))) _asbp_gameplay_gm)
  (bind _charactermovement (`Character.CharacterMovement` _asbp_character))
  (set `CharacterMovementComponent.MaxWalkSpeed` (`KismetMathLibrary.FClamp` (* (`CharacterMovementComponent.MaxWalkSpeed` _charactermovement) 1.01) 600.0 1200.0) _charactermovement)
  (`KismetSystemLibrary.Delay` 1.0)
  (`self.K2_DestroyActor`))

(fn `SpawnObstacle`
  (bind _returnvalue (`KismetMathLibrary.RandomFloatInRange` 0.0 1.0))
  (bind _returnvalue_2 (`KismetMathLibrary.RandomFloatInRange` 0.0 1.0))
  (bind _returnvalue_3 (`KismetMathLibrary.RandomFloatInRange` 0.0 1.0))
  (bind _returnvalue_4 (`SceneComponent.K2_GetComponentToWorld` (`self.Lane_0`)))
  (bind _returnvalue_5 (`SceneComponent.K2_GetComponentToWorld` (`self.Lane_1`)))
  (bind _returnvalue_6 (`SceneComponent.K2_GetComponentToWorld` (`self.Lane_2`)))
  ;[1 1 1] Lane 0
  (if (`KismetMathLibrary.InRange_FloatFloat` _returnvalue 0.0 0.4)
    (`|SpawnActorFromClass` "/Game/Blueprints/BP_ObstacleJump.BP_ObstacleJump_C" _returnvalue_4 "Undefined" "OverrideRootScale" null null)
    ;[1 1 1] Lane 1
    (if (`KismetMathLibrary.InRange_FloatFloat` _returnvalue_3 0.0 0.4) :!label _label
      (`|SpawnActorFromClass` "/Game/Blueprints/BP_ObstacleJump.BP_ObstacleJump_C" _returnvalue_5 "Undefined" "OverrideRootScale" null null)
      ;[1 1 1] Lane 1
      (if (`KismetMathLibrary.InRange_FloatFloat` _returnvalue_2 0.0 0.4) :!label _label_2
        (`|SpawnActorFromClass` "/Game/Blueprints/BP_ObstacleJump.BP_ObstacleJump_C" _returnvalue_6 "Undefined" "OverrideRootScale" null null)
        (elif (`KismetMathLibrary.InRange_FloatFloat` _returnvalue_2 0.4 0.5)
          (`|SpawnActorFromClass` "/Game/Blueprints/BP_Obstacle.BP_Obstacle_C" _returnvalue_6 "Undefined" "OverrideRootScale" null null)
          (elif (`KismetMathLibrary.InRange_FloatFloat` _returnvalue_2 0.5 0.95)
            (`|SpawnActorFromClass` "/Game/Blueprints/BP_Coin.BP_Coin_C" _returnvalue_6 "Undefined" "OverrideRootScale" null null)
            (elif (`KismetMathLibrary.InRange_FloatFloat` _returnvalue_2 0.95 0.975)
              (`|SpawnActorFromClass` "/Game/Blueprints/BP_Magnet.BP_Magnet_C" _returnvalue_6 "Undefined" "OverrideRootScale" null null)
              (elif (`KismetMathLibrary.InRange_FloatFloat` _returnvalue_2 0.975)
                (`|SpawnActorFromClass` "/Game/Blueprints/BP_Boots.BP_Boots_C" _returnvalue_6 "Undefined" "OverrideRootScale" null null))))))
      (elif (`KismetMathLibrary.InRange_FloatFloat` _returnvalue_3 0.4 0.5)
        (`|SpawnActorFromClass` "/Game/Blueprints/BP_Obstacle.BP_Obstacle_C" _returnvalue_5 "Undefined" "OverrideRootScale" null null)
        (goto _label_2)
        (elif (`KismetMathLibrary.InRange_FloatFloat` _returnvalue_3 0.5 0.95)
          (`|SpawnActorFromClass` "/Game/Blueprints/BP_Coin.BP_Coin_C" _returnvalue_5 "Undefined" "OverrideRootScale" null null)
          (goto _label_2)
          (elif (`KismetMathLibrary.InRange_FloatFloat` _returnvalue_3 0.95 0.975)
            (`|SpawnActorFromClass` "/Game/Blueprints/BP_Magnet.BP_Magnet_C" _returnvalue_5 "Undefined" "OverrideRootScale" null null)
            (goto _label_2)
            (elif (`KismetMathLibrary.InRange_FloatFloat` _returnvalue_3 0.975)
              (`|SpawnActorFromClass` "/Game/Blueprints/BP_Boots.BP_Boots_C" _returnvalue_5 "Undefined" "OverrideRootScale" null null)
              (goto _label_2))))))
    (elif (`KismetMathLibrary.InRange_FloatFloat` _returnvalue 0.4 0.5)
      (`|SpawnActorFromClass` "/Game/Blueprints/BP_Obstacle.BP_Obstacle_C" _returnvalue_4 "Undefined" "OverrideRootScale" null null)
      (goto _label)
      (elif (`KismetMathLibrary.InRange_FloatFloat` _returnvalue 0.5 0.95)
        (`|SpawnActorFromClass` "/Game/Blueprints/BP_Coin.BP_Coin_C" _returnvalue_4 "Undefined" "OverrideRootScale" null null)
        (goto _label)
        (elif (`KismetMathLibrary.InRange_FloatFloat` _returnvalue 0.95 0.975)
          (`|SpawnActorFromClass` "/Game/Blueprints/BP_Magnet.BP_Magnet_C" _returnvalue_4 "Undefined" "OverrideRootScale" null null)
          (goto _label)
          (elif (`KismetMathLibrary.InRange_FloatFloat` _returnvalue 0.975)
            (`|SpawnActorFromClass` "/Game/Blueprints/BP_Boots.BP_Boots_C" _returnvalue_4 "Undefined" "OverrideRootScale" null null)
            (goto _label)))))))

(fn `UserConstructionScript`)