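; In-game HUD actor that creates and manages the loading screen, pause menu, game over and main HUD widgets.
; Pause and game over events toggle widget visibility, game pause and input mode, leaving the mouse cursor shown even on unpause.
; Menu and restart events route through LoadLevel, which fades the loading screen and opens the main menu or current level when fading finishes.
; A separate event quits the game.
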(event `/Game/Blueprints/BP_HUD_Interface.Menu`
  ;[1 1 1] Main Menu
  (`self.LoadLevel` (`self.MainMenuLevelName`)))

(event `/Game/Blueprints/BP_HUD_Interface.QuitGame`
  ;[1 1 1] Quit Game
  (`KismetSystemLibrary.QuitGame` (`self.GetOwningPlayerController`) "Quit"))

(event `/Game/Blueprints/BP_HUD_Interface.StartGame`
  ;[1 1 1] Start Game
  (bind _returnvalue (`GameplayStatics.GetCurrentLevelName` true))
  (`self.LoadLevel` (`KismetStringLibrary.Conv_StringToName` _returnvalue)))

(event `self.ReceiveBeginPlay`
  ;[1 1 1] HUD Construct
  (`|ExecutionSequence`
    (:`then_0`
      (bind _returnvalue (`|CreateWidget` "/Game/Blueprints/WB_LoadingScreen.WB_LoadingScreen_C" (`self.GetOwningPlayerController`)))
      (bind _output_get (set `self.LoadingScreen` _returnvalue))
      (`/Game/Blueprints/WB_LoadingScreen.SetFade` _output_get 0.0)
      (`UserWidget.AddToViewport` _output_get 90000))
    (:`then_1`
      (bind _returnvalue_2 (`|CreateWidget` "/Game/Blueprints/WB_PauseMenu.WB_PauseMenu_C" (`self.GetOwningPlayerController`)))
      (bind _output_get_2 (set `self.PauseMenu` _returnvalue_2))
      (`Widget.SetVisibility` _output_get_2 "Collapsed")
      (`UserWidget.AddToViewport` _output_get_2 100))
    (:`then_2`
      (bind _returnvalue_3 (`|CreateWidget` "/Game/Blueprints/WB_GameOver.WB_GameOver_C" (`self.GetOwningPlayerController`)))
      (bind _output_get_3 (set `self.GameOverScreen` _returnvalue_3))
      (`UserWidget.AddToViewport` _output_get_3 500)
      (`Widget.SetVisibility` _output_get_3 "Collapsed"))
    (:`then_3`
      (bind _returnvalue_4 (`|CreateWidget` "/Game/Blueprints/WB_HUD.WB_HUD_C" (`self.GetOwningPlayerController`)))
      (bind _output_get_4 (set `self.HUD` _returnvalue_4))
      (`UserWidget.AddToViewport` _output_get_4 0))
    (:`then_4`
      (`WidgetBlueprintLibrary.SetInputMode_GameOnly` (`self.GetOwningPlayerController`)))))

(event `LoadLevel`
  (params (`Level Name` :type Name))
  ;[1 1 1] Load Level
  (if (!= `Level Name` "None")
    (bind _loadingscreen (`self.LoadingScreen`)
      (:`then`
        (`Widget.SetVisibility` _loadingscreen "SelfHitTestInvisible")
        (`/Game/Blueprints/WB_LoadingScreen.SetFade` _loadingscreen 1.0)
        (add `/Game/Blueprints/WB_LoadingScreen.DoneFading` _loadingscreen (delegate `LoadingLevel`)))
      (:`else`))))

(event `LoadingLevel`
  ;[1 1 1] Load Level
  (`GameplayStatics.OpenLevel` (stale `LoadLevel` `Level Name`)))

(event `/Game/Blueprints/BP_HUD_Interface.PauseGame`
  (params (Paused :type Boolean))
  (bind _returnvalue (`self.GetOwningPlayerController`))
  ;[1 1 1] Pause Menu
  (if Paused
    (`|ExecutionSequence`
      (:`then_0`
        (bind _pausemenu (`self.PauseMenu`)
          (:`then`
            (`Widget.SetVisibility` _pausemenu "Visible")
            (`WidgetBlueprintLibrary.SetInputMode_GameAndUIEx` (`self.GetOwningPlayerController`) _pausemenu "DoNotLock" false))
          (:`else`)))
      (:`then_1`
        (`GameplayStatics.SetGamePaused` true)
        (set `PlayerController.bShowMouseCursor` true (`self.GetOwningPlayerController`))))
    (else
      (`GameplayStatics.SetGamePaused` false)
      (set `PlayerController.bShowMouseCursor` true _returnvalue)
      (`WidgetBlueprintLibrary.SetInputMode_GameOnly` _returnvalue)
      (bind _pausemenu_2 (`self.PauseMenu`)
        (:`then`
          (`Widget.SetVisibility` _pausemenu_2 "Collapsed"))
        (:`else`)))))

(event `/Game/Blueprints/BP_HUD_Interface.GameOver`
  (bind _returnvalue (`self.GetOwningPlayerController`))
  (bind _gameoverscreen (`self.GameOverScreen`))
  ;[1 1 1] Game Over
  (`Widget.SetVisibility` _gameoverscreen "Visible")
  (`GameplayStatics.SetGamePaused` true)
  (set `PlayerController.bShowMouseCursor` true _returnvalue)
  (`WidgetBlueprintLibrary.SetInputMode_GameAndUIEx` _returnvalue _gameoverscreen "DoNotLock" false))

(fn `UserConstructionScript`)