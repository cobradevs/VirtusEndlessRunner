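; BP_Boots is a pickup that grants BP_Character a temporary jump boost.
; On overlap it plays a powerup sound, raises the character's JumpZVelocity and hides the boot mesh.
; After a ten-second delay it resets jump velocity to a hardcoded value on player character 0, then destroys itself.
; Overlap stays active during the delay, as only the mesh visibility changes.
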(event `self.ReceiveActorBeginOverlap`
  (params (OtherActor :type "Actor Object Reference"))
  (bind _asbp_character (cast `/Game/Blueprints/BP_Character` OtherActor))
  (`GameplayStatics.SpawnSound2D` "/Game/Audio/A_Powerup.A_Powerup" 1.0 1.0 0.0 null)
  (set `CharacterMovementComponent.JumpZVelocity` 800.0 (`Character.CharacterMovement` _asbp_character))
  (`SceneComponent.SetVisibility` (`self.BootMesh`) false false)
  (`KismetSystemLibrary.Delay` 10.0)
  (bind _asbp_character_2 (cast `/Game/Blueprints/BP_Character` (`GameplayStatics.GetPlayerCharacter` 0)))
  (set `CharacterMovementComponent.JumpZVelocity` 500.0 (`Character.CharacterMovement` _asbp_character_2))
  (`self.K2_DestroyActor`))

(fn `UserConstructionScript`)