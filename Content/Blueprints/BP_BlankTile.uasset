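; BP_BlankTile is a track tile, apparently for an endless runner, that reacts when the player character reaches its collision.
; On overlap it asks BP_GameplayGM to spawn a new tile and adds to the score using the game mode's multiplier.
; It also nudges the character's walk speed up by a small percentage within a clamped range, then destroys itself after a short delay.
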(event `self.Collision.OnComponentBeginOverlap`
  (params (OverlappedComponent :type "PrimitiveComponent Object Reference") (OtherActor :type "Actor Object Reference") (OtherComp :type "PrimitiveComponent Object Reference") (OtherBodyIndex :type Integer) (bFromSweep :type Boolean) (SweepResult :type "HitResult Structure (by ref)"))
  (bind _asbp_character (cast `/Game/Blueprints/BP_Character` OtherActor))
  (bind _asbp_gameplay_gm (cast `/Game/Blueprints/BP_GameplayGM` (`GameplayStatics.GetGameMode`)))
  (`/Game/Blueprints/BP_GameplayGM.SpawnTile` _asbp_gameplay_gm)
  (set `/Game/Blueprints/BP_GameplayGM.Score` (+ (`/Game/Blueprints/BP_GameplayGM.Score` _asbp_gameplay_gm) (* 1 (`/Game/Blueprints/BP_GameplayGM.ScoreMultiplier` _asbp_gameplay_gm))) _asbp_gameplay_gm)
  (bind _charactermovement (`Character.CharacterMovement` _asbp_character))
  (set `CharacterMovementComponent.MaxWalkSpeed` (`KismetMathLibrary.FClamp` (* (`CharacterMovementComponent.MaxWalkSpeed` _charactermovement) 1.01) 600.0 1200.0) _charactermovement)
  (`KismetSystemLibrary.Delay` 1.0)
  (`self.K2_DestroyActor`))

(fn `UserConstructionScript`)