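; Gameplay game mode that builds a chained tile track and handles game over with high score saving.
; On BeginPlay it spawns one blank tile, then ten master tiles, each placed at the previous tile's SpawnPoint location through NextSpawnPoint.
; GameOver shows the HUD message, then updates the HighScore save slot if the score beats the stored value, or creates the save if none exists.
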(event `self.ReceiveBeginPlay`
  (`self.SpawnBlankTile`)
  (for _ (range 10)
    (`self.SpawnTile`)))

(event `GameOver`
  (message `/Game/Blueprints/BP_HUD_Interface.GameOver` (`PlayerController.GetHUD` (`GameplayStatics.GetPlayerController` 0)))
  (bind _returnvalue (`GameplayStatics.DoesSaveGameExist` "Highscore"))
  (if _returnvalue
    (bind _returnvalue_2 (`GameplayStatics.LoadGameFromSlot` "HighScore"))
    (bind _asbp_save_game (cast `/Game/Blueprints/BP_SaveGame` _returnvalue_2))
    (set `self.SaveGame` _asbp_save_game)
    (if (> (`self.Score`) (`/Game/Blueprints/BP_SaveGame.HighScore` (`self.SaveGame`)))
      (set `/Game/Blueprints/BP_SaveGame.HighScore` (`self.Score`) (`self.SaveGame`))
      (`GameplayStatics.SaveGameToSlot` (`self.SaveGame`) "HighScore"))
    (else
      (bind _returnvalue_3 (`GameplayStatics.CreateSaveGameObject` "/Game/Blueprints/BP_SaveGame.BP_SaveGame_C"))
      (set `/Game/Blueprints/BP_SaveGame.HighScore` (`self.Score`) _returnvalue_3)
      (`GameplayStatics.SaveGameToSlot` _returnvalue_3 "HighScore"))))

(fn `SpawnBlankTile`
  (bind _returnvalue (`|SpawnActorFromClass` "/Game/Blueprints/BP_BlankTile.BP_BlankTile_C" (`self.NextSpawnPoint`) "Undefined" "OverrideRootScale" null null))
  (set `self.NextSpawnPoint` (`KismetMathLibrary.MakeTransform` (`SceneComponent.K2_GetComponentLocation` (`/Game/Blueprints/BP_BlankTile.SpawnPoint` _returnvalue)))))

(fn `SpawnTile`
  (bind _returnvalue (`|SpawnActorFromClass` "/Game/Blueprints/BP_MasterTile.BP_MasterTile_C" (`self.NextSpawnPoint`) "Undefined" "OverrideRootScale" null null))
  (set `self.NextSpawnPoint` (`KismetMathLibrary.MakeTransform` (`SceneComponent.K2_GetComponentLocation` (`/Game/Blueprints/BP_MasterTile.SpawnPoint` _returnvalue)))))

(fn `UserConstructionScript`)